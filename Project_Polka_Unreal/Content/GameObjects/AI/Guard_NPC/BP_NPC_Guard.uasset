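; Guard NPC Blueprint that exposes six body-part target points (head, body, arms, legs) for combat targeting.
; On BeginPlay it builds the target list and an enum lookup map, and every Tick it caches the combat lock point's world location.
; An interface event receives a reticle point, switches to any closer body target and its mapped enum, then refreshes the stored target world locations.
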(event EventBeginPlay
  (CallFunction|SetUp))

(event Collision|EventActorBeginOverlap
  (params (OtherActor :type Actor%20Object%20Reference)))

(event EventTick
  (params (DeltaSeconds :type Float%20%28single-precision%29))
  (CallFunction|UpdateCombatLockPointLocation))

(event EventInterfaceChangeCombatTarget
  (params (CombatReticlePoint :type Vector :default "0, 0, 0"))
  (CallFunction|ChangeOtherCombatTarget CombatReticlePoint)
  (CallFunction|UpdateTargetLocationInfo))

(fn ConstructionScript)

(fn UpdateCombatLockPointLocation
  (Variables|/Game/GameObjects/AI/BP_NPC.BP_NPC_C|SetcombatLockPointLocation self (Transformation|GetWorldLocation (Variables|Default|GetCombatLockLocation))))

(fn ChangeOtherCombatTarget
  (params (targettingPoint :type Vector))
  (for _array_element (Variables|Default|GetcombatTargetsOnSelf)
    (if (< (Math|Vector|Distance(Vector) targettingPoint (Transformation|GetWorldLocation _array_element)) (Math|Vector|Distance(Vector) targettingPoint (Transformation|GetWorldLocation (Variables|Default|GetclosestTargetOnSelf))))
      (bind _output_get (Variables|Default|SetclosestTargetOnSelf _array_element))
      (if (.ReturnValue (Utilities|Map|Find (Variables|Default|GetmapTargetToEnumTarget) _output_get))
        (Variables|Default|SetotherCombatTargets (.Value (Utilities|Map|Find (Variables|Default|GetmapTargetToEnumTarget) _output_get)))
        (else
          (Development|PrintString (Utilities|String|Append (Utilities|GetDisplayName self) " - Didn't find combat target in the map")))))))

(fn SetUp
  (bind _targethead (Variables|Default|GetTargetHead))
  (bind _targetbody (Variables|Default|GetTargetBody))
  (bind _targetrightarm (Variables|Default|GetTargetRightArm))
  (bind _targetleftarm (Variables|Default|GetTargetLeftArm))
  (bind _targetrightleg (Variables|Default|GetTargetRightLeg))
  (bind _targetleftleg (Variables|Default|GetTargetLeftLeg))
  (Utilities|FlowControl|Sequence
    (:then_0
      (Variables|Default|SetclosestTargetOnSelf _targethead)
      (Variables|Default|SetcombatTargetsOnSelf (Utilities|Array|MakeArray _targethead _targetbody _targetrightarm _targetleftarm _targetrightleg _targetleftleg)))
    (:then_1
      (Variables|Default|SetmapTargetToEnumTarget (Utilities|Map|MakeMap _targethead "NewEnumerator0" _targetbody "NewEnumerator1" _targetrightarm "NewEnumerator2" _targetleftarm "NewEnumerator3" _targetrightleg "NewEnumerator4" _targetleftleg "NewEnumerator5")))))

(fn UpdateTargetLocationInfo
  (bind _targetlocations (Variables|Default|GettargetLocations))
  (Utilities|Array|Clear _targetlocations)
  (for _array_element (Variables|Default|GetcombatTargetsOnSelf)
    (Utilities|Array|Add _targetlocations (Transformation|GetWorldLocation _array_element))))