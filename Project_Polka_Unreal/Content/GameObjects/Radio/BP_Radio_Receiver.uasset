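; In-world radio receiver that plays one of two stations broadcast by the level's BP_Radio_Transmitter, found at BeginPlay.
; While on, Tick compares its audio with the transmitter's current song and, on mismatch, plays that song from the station's time to stay in sync.
; InteractE cycles stations and InteractF toggles power, both only with a transmitter present.
; Powering off clears the sound, so powering on resyncs to the broadcast.
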(event EventBeginPlay
  (bind _returnvalue (Actor|GetActorOfClass "/Game/GameObjects/Radio/BP_Radio_Transmitter.BP_Radio_Transmitter_C"))
  (if (== (Utilities|GetClass _returnvalue) "/Game/GameObjects/Radio/BP_Radio_Transmitter.BP_Radio_Transmitter_C")
    (Variables|Default|SetradioTransmitter _returnvalue)
    (Variables|Default|SethasRadioTransmitter true)
    (else
      (Development|PrintString "No radio transmitter")
      (if (Variables|Default|GetradioIsOn)
        (CallFunction|TurnRadioonOff)))))

(event Collision|EventActorBeginOverlap
  (params (OtherActor :type Actor%20Object%20Reference)))

(event EventTick
  (params (DeltaSeconds :type Float%20%28single-precision%29))
  (bind _currentradiostation (Variables|Default|GetcurrentRadioStation))
  (if (Variables|Default|GetradioIsOn)
    (Utilities|FlowControl|Sequence
      (:then_0
        (if (== _currentradiostation 0)
          (bind _songchangebool (CallFunction|CheckforSongChangeStationOne))
          (if _songchangebool
            (CallFunction|ChangeRadioSongStationOne))))
      (:then_1
        (if (== _currentradiostation 1)
          (bind _songchangebool_2 (CallFunction|CheckforSongChangeStationTwo))
          (if _songchangebool_2
            (CallFunction|ChangeRadioSongStationTwo)))))))

(event EventInteractF
  (if (Variables|Default|GethasRadioTransmitter)
    (CallFunction|TurnRadioonOff)))

(event EventInteractE
  (if (Variables|Default|GethasRadioTransmitter)
    (CallFunction|ChangeRadioStation)))

(fn ConstructionScript)

(fn CheckforSongChangeStationOne
  (bind _radiotransmitter (Variables|Default|GetradioTransmitter))
  (return (!= (Utilities|Array|Get(acopy) (Variables|/Game/GameObjects/Radio/BP_Radio_Transmitter.BP_Radio_Transmitter_C|GetStationOneAudioClips _radiotransmitter) (Variables|/Game/GameObjects/Radio/BP_Radio_Transmitter.BP_Radio_Transmitter_C|GetStationOneSong _radiotransmitter)) (Variables|/Script/Engine.AudioComponent|GetSound (Variables|Default|GetAudio)))))

(fn ChangeRadioSongStationOne
  (bind _radiotransmitter (Variables|Default|GetradioTransmitter))
  (Audio|Components|Audio|SetSound (Variables|Default|GetAudio) (Utilities|Array|Get(acopy) (Variables|/Game/GameObjects/Radio/BP_Radio_Transmitter.BP_Radio_Transmitter_C|GetStationOneAudioClips _radiotransmitter) (Variables|/Game/GameObjects/Radio/BP_Radio_Transmitter.BP_Radio_Transmitter_C|GetStationOneSong _radiotransmitter)))
  (Audio|Components|Audio|Play (Variables|Default|GetAudio) (Variables|/Game/GameObjects/Radio/BP_Radio_Transmitter.BP_Radio_Transmitter_C|GetStationOneTime _radiotransmitter)))

(fn CheckforSongChangeStationTwo
  (bind _radiotransmitter (Variables|Default|GetradioTransmitter))
  (return (!= (Utilities|Array|Get(acopy) (Variables|/Game/GameObjects/Radio/BP_Radio_Transmitter.BP_Radio_Transmitter_C|GetStationTwoAudioClips _radiotransmitter) (Variables|/Game/GameObjects/Radio/BP_Radio_Transmitter.BP_Radio_Transmitter_C|GetStationTwoSong _radiotransmitter)) (Variables|/Script/Engine.AudioComponent|GetSound (Variables|Default|GetAudio)))))

(fn ChangeRadioSongStationTwo
  (bind _radiotransmitter (Variables|Default|GetradioTransmitter))
  (Audio|Components|Audio|SetSound (Variables|Default|GetAudio) (Utilities|Array|Get(acopy) (Variables|/Game/GameObjects/Radio/BP_Radio_Transmitter.BP_Radio_Transmitter_C|GetStationTwoAudioClips _radiotransmitter) (Variables|/Game/GameObjects/Radio/BP_Radio_Transmitter.BP_Radio_Transmitter_C|GetStationTwoSong _radiotransmitter)))
  (Audio|Components|Audio|Play (Variables|Default|GetAudio) (Variables|/Game/GameObjects/Radio/BP_Radio_Transmitter.BP_Radio_Transmitter_C|GetStationTwoTime _radiotransmitter)))

(fn ChangeRadioStation
  (if (Variables|Default|GetradioIsOn)
    (Development|PrintString "Changed Radio Station")
    (if (> (+ (Variables|Default|GetcurrentRadioStation) 1) (- (Variables|/Game/GameObjects/Radio/BP_Radio_Transmitter.BP_Radio_Transmitter_C|GetTotalAmountOfStations (Variables|Default|GetradioTransmitter)) 1))
      (Variables|Default|SetcurrentRadioStation "NewEnumerator0")
      (else
        (Variables|Default|SetcurrentRadioStation (Utilities|Enum|ByteToEnumRadioStations (+ (Variables|Default|GetcurrentRadioStation) 1)))))))

(fn TurnRadioonOff
  (bind _audio (Variables|Default|GetAudio))
  (if (== (Variables|Default|GetradioIsOn) false)
    (Variables|Default|SetradioIsOn true)
    (Development|PrintString "Radio Turned On")
    (else
      (Variables|Default|SetradioIsOn false)
      (Audio|Components|Audio|SetSound _audio 0)
      (Audio|Components|Audio|Stop _audio)
      (Development|PrintString "Radio Turned Off"))))