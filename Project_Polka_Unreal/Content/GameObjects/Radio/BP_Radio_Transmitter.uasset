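; Radio transmitter Blueprint that keeps a running playlist position and playback time for two radio stations.
; Each Tick it advances both station timers and compares them with the duration of the current clip in each station's audio array.
; When a clip's time is exceeded, that station moves to the next index, wrapping to the first after the last, and resets its timer.
; It only tracks state and plays no audio itself.
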(event EventBeginPlay
  (Variables|Default|SetTotalAmountOfStations 2))

(event Collision|EventActorBeginOverlap
  (params (OtherActor :type Actor%20Object%20Reference)))

(event EventTick
  (params (DeltaSeconds :type Float%20%28single-precision%29))
  (bind (_timestampstationone _timestampstationtwo) (CallFunction|AddtoStations'Time DeltaSeconds))
  (bind (_songdurationstationone _songpositioninarraystationone _songdurationstationtwo _songpositioninarraystationtwo) (CallFunction|GetCurrentStations'Songs))
  (bind (_songisoverstationone _isthelastsongstationone _currentpositionplusonestationone _songisoverstationtwo _isthelastsongstationtwo _currentpositionplusonestationtwo) (CallFunction|CompareTimeandSongPositions _songdurationstationone _timestampstationone _songpositioninarraystationone _songdurationstationtwo _timestampstationtwo _songpositioninarraystationtwo))
  ;[0.3608 0.2275 0.1686] Station One
  (if _songisoverstationone
    (if _isthelastsongstationone
      (Variables|Default|SetStationOneSong 0)
      (else
        (Variables|Default|SetStationOneSong _currentpositionplusonestationone)))
    (Variables|Default|SetStationOneTime 0.0))
  ;[0.3608 0.2275 0.1686] Station Two
  (if _songisoverstationtwo
    (if _isthelastsongstationtwo
      (Variables|Default|SetStationTwoSong 0)
      (else
        (Variables|Default|SetStationTwoSong _currentpositionplusonestationtwo)))
    (Variables|Default|SetStationTwoTime 0.0)))

(fn ConstructionScript)

(fn AddtoStations'Time
  (params (DeltaTime :type Float%20%28double-precision%29))
  (Variables|Default|SetStationOneTime (+ DeltaTime (Variables|Default|GetStationOneTime)))
  (Variables|Default|SetStationTwoTime (+ DeltaTime (Variables|Default|GetStationTwoTime)))
  (return (+ DeltaTime (Variables|Default|GetStationOneTime)) (+ DeltaTime (Variables|Default|GetStationTwoTime))))

(fn GetCurrentStations'Songs
  (bind _stationoneaudioclips (Variables|Default|GetStationOneAudioClips))
  (bind _stationtwoaudioclips (Variables|Default|GetStationTwoAudioClips))
  (return (Variables|/Script/Engine.SoundBase|GetDuration (Utilities|Array|Get(acopy) _stationoneaudioclips (Variables|Default|GetStationOneSong))) (- (Utilities|Array|Length _stationoneaudioclips) 1) (Variables|/Script/Engine.SoundBase|GetDuration (Utilities|Array|Get(acopy) _stationtwoaudioclips (Variables|Default|GetStationTwoSong))) (- (Utilities|Array|Length _stationtwoaudioclips) 1)))

(fn CompareTimeandSongPositions
  (params (SongDurationStationOne :type Float%20%28double-precision%29) (TimeStampStationOne :type Float%20%28double-precision%29) (SongPositionInArrayStationOne :type Integer) (SongDurationStationTwo :type Float%20%28double-precision%29) (TimeStampStationTwo :type Float%20%28double-precision%29) (SongPositionInArrayStationTwo :type Integer))
  (bind _stationonesong (Variables|Default|GetStationOneSong))
  (bind _stationtwosong (Variables|Default|GetStationTwoSong))
  (bind _returnvalue (+ _stationonesong 1))
  (bind _returnvalue_2 (+ _stationtwosong 1))
  (return (< SongDurationStationOne TimeStampStationOne) (< SongPositionInArrayStationOne _returnvalue) _returnvalue (< SongDurationStationTwo TimeStampStationTwo) (< SongPositionInArrayStationTwo _returnvalue_2) _returnvalue_2))